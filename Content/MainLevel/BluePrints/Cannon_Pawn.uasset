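; Player-possessed cannon pawn that launches a StuntMan using a two-press timing meter, with max power and swing speed read from the game instance.
; Tick swings the barrel between pitch limits until StopMeter locks rotation, then bounces a counter that drives the power value exposed through GetLerpValue.
; A second press locks power, and a DoOnce spawns the StuntMan at the Sphere and launches it with power derived from the counter.
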(event `self.ReceiveBeginPlay`
  (`self.Start`)
  (`Controller.Possess` (`GameplayStatics.GetPlayerController` 0) self)
  (set `self.LockRotation` false)
  (set `self.LockPower` false))

(event `self.ReceiveTick`
  (params (DeltaSeconds :type "Float (single-precision)"))
  (bind _time (`self.Time`))
  (bind (_returnvalue_roll _returnvalue_pitch) (`KismetMathLibrary.BreakRotator` (`SceneComponent.K2_GetComponentRotation` (`self.Cannon`))))
  (bind _returnvalue (+ _time 1))
  (bind _returnvalue_2 (`KismetMathLibrary.Lerp` 0.5 (`self.MaxPower`) (`KismetMathLibrary.Conv_IntToDouble` (mod _returnvalue 30))))
  (if (`self.LockRotation`)
    (if (`self.LockPower`)
      (`/Engine/EditorBlueprintResources/StandardMacros.DoOnce` false
        (:`Completed`
          (bind _output_get (set `self.Power` _returnvalue_2))
          (bind _returnvalue_3 (`|SpawnActorFromClass` "/Game/MainLevel/BluePrints/StuntMan.StuntMan_C" (`KismetMathLibrary.Conv_VectorToTransform` (`SceneComponent.K2_GetComponentLocation` (`self.Sphere`))) "AdjustIfPossibleButAlwaysSpawn" "MultiplyWithRoot" null null))
          (`/Game/MainLevel/BluePrints/StuntMan.Launch` _returnvalue_3 _output_get)))
      (else
        (if (and (< _time 29) (not (`self.CountingDown`)))
          (bind _output_get_2 (set `self.Time` _returnvalue))
          (else
            (bind _output_get_3 (set `self.Time` (- _time 1)))
            (bind _returnvalue_4 (!= _output_get_3 0))
            (if _returnvalue_4
              (set `self.CountingDown` _returnvalue_4)
              (else
                (set `self.CountingDown` false)))))
        (set `self.lerpValue` (/ _returnvalue_2 (* (`self.MaxPower`) 30.0)))))
    (elif (`self.MovingUp`)
      (`SceneComponent.K2_AddRelativeRotation` (`self.Cannon`) (* (`self.PositiveRotation`) (`self.speedMulti`)) false false)
      (if (>= _returnvalue_pitch 90.0)
        (set `self.MovingUp` false))
      (else
        (`SceneComponent.K2_AddRelativeRotation` (`self.Cannon`) (* (`self.NegativeRotation`) (`self.speedMulti`)) false false)
        (if (<= _returnvalue_pitch 35.0)
          (set `self.MovingUp` true))))))

(event `InputAction|StopMeter`
  (params (Key :type "Key Structure"))
  (:`Pressed`
    (if (`self.LockRotation`)
      (set `self.LockPower` true)
      (else
        (set `self.LockRotation` true)))))

(fn `getLerpValue`
  (returns (NewParam :type "Float (double-precision)"))
  (return (`self.lerpValue`)))

(fn `Start`
  (bind _asstunt_man_instance (cast `/Game/StuntMan_Instance` (`GameplayStatics.GetGameInstance`)))
  (bind _output_get (set `self.As Stunt Man Instance` _asstunt_man_instance))
  (`|ExecutionSequence`
    (:`then_0`
      (bind _power (`/Game/StuntMan_Instance.getPower` _output_get))
      (bind _output_get_2 (set `self.MaxPower` _power))
      (`KismetSystemLibrary.PrintString` (`KismetStringLibrary.Conv_DoubleToString` _output_get_2)))
    (:`then_1`
      (bind _speedmulti (`/Game/StuntMan_Instance.getSpeed` _output_get))
      (bind _output_get_3 (set `self.speedMulti` _speedmulti))
      (`KismetSystemLibrary.PrintString` (`KismetStringLibrary.Conv_DoubleToString` _output_get_3)))))

(fn `UserConstructionScript`)