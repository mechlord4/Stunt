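; MainLevelACtor is an actor that sets up the score HUD and handles the pause key for the main level.
; BeginPlay adds a Score_WBP widget to the viewport.
; Tab passes IsPaused to SetGamePaused, though comparing the flag with itself always yields false.
; It also adds a new Pause_WBP on each press, switches input to UI-only, and sets cursor visibility from SetGamePaused's return value.
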(event `self.ReceiveBeginPlay`
  (bind _returnvalue (`|CreateWidget` "/Game/MainLevel/Widgets/Score_WBP.Score_WBP_C"))
  (`UserWidget.AddToViewport` _returnvalue 0))

(event `Key|Tab`
  (params (Key :type "Key Structure"))
  (bind _ispaused (`self.isPaused`))
  (:`Pressed`
    (bind _output_get (set `self.isPaused` (!= _ispaused _ispaused)))
    (bind _returnvalue (`GameplayStatics.SetGamePaused` _output_get))
    (bind _returnvalue_2 (`|CreateWidget` "/Game/MainLevel/Widgets/Pause_WBP.Pause_WBP_C"))
    (`UserWidget.AddToViewport` _returnvalue_2 0)
    (`WidgetBlueprintLibrary.SetInputMode_UIOnlyEx` null _returnvalue_2)
    (set `PlayerController.bShowMouseCursor` _returnvalue (`GameplayStatics.GetPlayerController` 0))))

(fn `UserConstructionScript`)