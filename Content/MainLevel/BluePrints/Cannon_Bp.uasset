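; Cannon Blueprint with a two-stage stop meter for setting aim angle, then power; it contains no firing logic.
; BeginPlay calls Possess on player controller 0 and clears both locks.
; Tick swings the Cannon's pitch between roughly 0 and 90 degrees until the first StopMeter press locks rotation.
; A counter then increments until the second press, after which a modulo-driven Lerp sets Power from MaxPower.
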(event `self.ReceiveBeginPlay`
  (`Controller.Possess` (`GameplayStatics.GetPlayerController` 0) null)
  (set `self.LockRotation` false)
  (set `self.LockPower` false))

(event `self.ReceiveTick`
  (params (DeltaSeconds :type "Float (single-precision)"))
  (bind (_returnvalue_roll _returnvalue_pitch) (`KismetMathLibrary.BreakRotator` (`SceneComponent.K2_GetComponentRotation` (`self.Cannon`))))
  (if (`self.LockRotation`)
    (if (`self.LockPower`)
      (set `self.Power` (`KismetMathLibrary.Lerp` 0.0 (`self.MaxPower`) (`KismetMathLibrary.Conv_IntToDouble` (mod (stale _result) 7))))
      (else
        (bind _result (`/Engine/EditorBlueprintResources/StandardMacros.IncrementInt` (`self.Time`)))))
    (elif (`self.MovingUp`)
      (`SceneComponent.K2_AddRelativeRotation` (`self.Cannon`) (struct :`Pitch` 10.0) false false)
      (if (>= _returnvalue_pitch 90.0)
        (set `self.MovingUp` false))
      (else
        (`SceneComponent.K2_AddRelativeRotation` (`self.Cannon`) (struct :`Pitch` -10.0) false false)
        (if (<= _returnvalue_pitch 0.0)
          (set `self.MovingUp` true))))))

(event `InputAction|StopMeter`
  (params (Key :type "Key Structure"))
  (:`Pressed`
    (if (`self.LockRotation`)
      (set `self.LockPower` true)
      (else
        (set `self.LockRotation` true)))))

(fn `UserConstructionScript`)