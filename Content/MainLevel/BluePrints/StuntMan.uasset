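; StuntMan is the player-possessed stuntman, launched by an impulse on its skeletal mesh and tracked until the run ends.
; Construction copies the rocket jump count from Stuntman_GameMode.
; Tick exposes distance from world origin and a moving flag based on Y/Z velocity.
; Each motionless tick restarts a two-second retriggerable delay that, on completion, opens the RunOver widget with cursor and UI-only input.
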(event `self.ReceiveBeginPlay`
  (`Controller.Possess` (`GameplayStatics.GetPlayerController` 0) self))

(event `self.ReceiveTick`
  (params (DeltaSeconds :type "Float (single-precision)"))
  (bind _returnvalue (`GameplayStatics.GetPlayerController` 0))
  (bind (_returnvalue_x _returnvalue_y _returnvalue_z) (`KismetMathLibrary.BreakVector` (`self.GetVelocity`)))
  (bind _output_get (set `self.isMoving` (or (!= _returnvalue_y 0.0) (!= _returnvalue_z 0.0))))
  (set `self.Distance` (`KismetMathLibrary.Vector_Distance` (0.0 0.0 0.0) (`SceneComponent.K2_GetComponentLocation` (`self.SkeletalMesh`))))
  (if (not _output_get)
    (`KismetSystemLibrary.RetriggerableDelay` 2.0)
    (bind _returnvalue_2 (`|CreateWidget` "/Game/MainLevel/RunOver_WBP.RunOver_WBP_C"))
    (`UserWidget.AddToViewport` _returnvalue_2 0)
    (`WidgetBlueprintLibrary.SetInputMode_UIOnlyEx` _returnvalue _returnvalue_2 "LockAlways")
    (set `PlayerController.bShowMouseCursor` true _returnvalue)))

(fn `getDistance`
  (returns (Distance :type "Float (double-precision)"))
  (return (`self.Distance`)))

(fn `getMoving`
  (returns (isMoving :type Boolean))
  (return (`self.isMoving`)))

(fn `Launch`
  (params (Power :type "Float (double-precision)"))
  (`PrimitiveComponent.AddImpulse` (`self.SkeletalMesh`) (`KismetMathLibrary.Conv_DoubleToVector` Power) "None" false))

(fn `UserConstructionScript`
  (bind _asstuntman_game_mode (cast `/Game/Stuntman_GameMode` (`GameplayStatics.GetGameMode`)))
  (bind _rocketjumps (`/Game/Stuntman_GameMode.getRocketJumps` _asstuntman_game_mode))
  (set `self.RocketJumps` _rocketjumps))